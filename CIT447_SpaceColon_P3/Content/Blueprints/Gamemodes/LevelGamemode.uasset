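; Level game mode that sets up the player's UI and respawns the main character when it is destroyed.
; BeginPlay and Respawn share one setup path: bind the character's OnDestroyed, add the main level and opening widgets, pause, and set cursor visibility from the pause result.
; On destruction, it waits briefly, spawns and possesses a new character at SpawnTransform, then reruns that setup, creating both widgets and pausing again.
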(event `Respawn`
  ;[0 0.5 1] On Destroy, Respawn (Jack)
  (bind _asmain_character (cast `/Game/Blueprints/PlayerCharacter/Blueprints/Character/Blueprints/MainCharacter` (`GameplayStatics.GetPlayerCharacter` 0) :!label _label))
  (add `self.OnDestroyed` _asmain_character (delegate `OnDestroyed_Event_0`))
  (bind _returnvalue (`|CreateWidget` "/Game/UI/MainLevelWidget_UI.MainLevelWidget_UI_C"))
  (bind _output_get (set `self.MainLevelWidget` _returnvalue))
  (`UserWidget.AddToViewport` _output_get 0)
  (bind _returnvalue_2 (`|CreateWidget` "/Game/UI/OpeningWidget_UI.OpeningWidget_UI_C"))
  (bind _output_get_2 (set `self.OpeningWidget` _returnvalue_2))
  (`UserWidget.AddToViewport` _output_get_2 0)
  (bind _returnvalue_3 (`GameplayStatics.SetGamePaused` true))
  (set `PlayerController.bShowMouseCursor` _returnvalue_3 (`GameplayStatics.GetPlayerController` 0)))

(event `self.ReceiveBeginPlay`
  ;[0 0.5 1] On Destroy, Respawn (Jack)
  (goto _label))

(event `OnDestroyed_Event_0` :!signature `self.OnDestroyed`
  (params (DestroyedActor :type "Actor Object Reference"))
  ;[0 0.5 1] On Destroy, Respawn (Jack)
  (`KismetSystemLibrary.Delay` 2.0)
  (bind _returnvalue (`|SpawnActorFromClass` "/Game/Blueprints/PlayerCharacter/Blueprints/Character/Blueprints/MainCharacter.MainCharacter_C" (`self.Spawn Transform`) "Undefined" "OverrideRootScale" null null))
  (`Controller.Possess` (`GameplayStatics.GetPlayerController` 0) _returnvalue)
  (`self.Respawn`))

(fn `UserConstructionScript`)