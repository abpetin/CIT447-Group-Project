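; Player controller Blueprint that toggles the exit menu and game pause from the OpenMenu input action.
; Each press flips IsMenuOpen, and a true result removes all top-level ExitMenuWidget_UI widgets and unpauses the game.
; A false result creates and displays a new menu widget, pauses the game and shows the mouse cursor, which the closing branch leaves visible.
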(event `InputAction|OpenMenu`
  (params (Key :type "Key Structure"))
  ;[1 1 1] Univeral Opening and Closing of the Menu
  (:`Pressed`
    (bind _output_get (set `self.isMenuOpen` (not (`self.isMenuOpen`))))
    (if _output_get
      (bind _foundwidgets (`WidgetBlueprintLibrary.GetAllWidgetsOfClass` "/Game/UI/ExitMenuWidget_UI.ExitMenuWidget_UI_C"))
      (`Widget.RemoveFromParent` _foundwidgets)
      (`GameplayStatics.SetGamePaused` false)
      (else
        (bind _returnvalue (`|CreateWidget` "/Game/UI/ExitMenuWidget_UI.ExitMenuWidget_UI_C"))
        (bind _output_get_2 (set `self.ExitMenuWidget` _returnvalue))
        (`UserWidget.AddToViewport` _output_get_2 0)
        (`GameplayStatics.SetGamePaused` true)
        (set `PlayerController.bShowMouseCursor` true (`GameplayStatics.GetPlayerController` 0))))))

(fn `UserConstructionScript`)