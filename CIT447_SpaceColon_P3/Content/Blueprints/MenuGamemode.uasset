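; Game mode for the menu levels, which puts up the UI screen that matches the current level.
; On BeginPlay it calls SetWidgetFunction, then shows the mouse cursor for the first player controller.
; SetWidgetFunction compares the current level name against the main menu, win and lose levels, then creates and stores the matching widget and adds it to the viewport.
; Any other level name falls back to the credits widget.
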(event `self.ReceiveBeginPlay`
  (`self.SetWidgetFunction`)
  (set `PlayerController.bShowMouseCursor` true (`GameplayStatics.GetPlayerController` 0)))

(fn `SetWidgetFunction`
  ;[0 0.1107 1] YAAAY FUNCTIONS--- ARCHIE ---
  (bind _returnvalue (`GameplayStatics.GetCurrentLevelName` true))
  (if (`KismetStringLibrary.EqualEqual_StrStr` _returnvalue (`self.MainMenuLevel`))
    (bind _returnvalue_2 (`|CreateWidget` "/Game/UI/MainLevelWidget_UI.MainLevelWidget_UI_C"))
    (bind _output_get (set `self.MainLevelWidget` _returnvalue_2))
    (`UserWidget.AddToViewport` _output_get 0)
    (elif (`KismetStringLibrary.EqualEqual_StrStr` _returnvalue (`self.WinLevel`))
      (bind _returnvalue_3 (`|CreateWidget` "/Game/UI/WinLevelWidget_UI.WinLevelWidget_UI_C"))
      (bind _output_get_2 (set `self.WinLevelWidget` _returnvalue_3))
      (`UserWidget.AddToViewport` _output_get_2 0)
      (elif (`KismetStringLibrary.EqualEqual_StrStr` _returnvalue (`self.LoseLevel`))
        (bind _returnvalue_4 (`|CreateWidget` "/Game/UI/LoseLevelWidget_UI.LoseLevelWidget_UI_C"))
        (bind _output_get_3 (set `self.LoseLevelWidget` _returnvalue_4))
        (`UserWidget.AddToViewport` _output_get_3 0)
        (else
          (bind _returnvalue_5 (`|CreateWidget` "/Game/UI/CreditsWidget_UI.CreditsWidget_UI_C"))
          (bind _output_get_4 (set `self.CreditLevelWidget` _returnvalue_5))
          (`UserWidget.AddToViewport` _output_get_4 0))))))

(fn `UserConstructionScript`)