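; MainCharacter is the player character Blueprint, handling mouse look and planar movement.
; Yaw and Pitch axes rotate the controller, while Forward and Strafe move along directions derived from control yaw only, keeping movement on the ground plane.
; On BeginPlay, both arm chains from the clavicles down switch to physics simulation, leaving the arms physics-driven on the skeletal mesh.
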(event `InputAxis|Yaw`
  (params (AxisValue :type "Float (single-precision)"))
  ;[1 1 1] mouse-based view rotation
  (`self.AddControllerYawInput` AxisValue))

(event `InputAxis|Pitch`
  (params (AxisValue :type "Float (single-precision)"))
  ;[1 1 1] mouse-based view rotation
  (`self.AddControllerPitchInput` AxisValue))

(event `self.ReceiveBeginPlay`
  ;[1 1 1] Physics
  (`SkeletalMeshComponent.SetAllBodiesBelowSimulatePhysics` (`self.Mesh`) "clavicle_l" true true)
  (`SkeletalMeshComponent.SetAllBodiesBelowSimulatePhysics` (`self.Mesh`) "clavicle_r" true true))

(event `InputAxis|Forward`
  (params (AxisValue :type "Float (single-precision)"))
  ;[1 1 1] movement
  (`self.AddMovementInput` (`KismetMathLibrary.GetForwardVector` (`KismetMathLibrary.MakeRotator` 0.0 0.0 (.yaw (`self.GetControlRotation`)))) AxisValue))

(event `InputAxis|Strafe`
  (params (AxisValue :type "Float (single-precision)"))
  ;[1 1 1] movement
  (`self.AddMovementInput` (`KismetMathLibrary.GetRightVector` (`KismetMathLibrary.MakeRotator` 0.0 0.0 (.yaw (`self.GetControlRotation`)))) AxisValue))

(fn `UserConstructionScript`)