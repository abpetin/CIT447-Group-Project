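; Player controller that handles the level menu and mouse cursor toggles from input actions.
; OpenMenu flips IsMenuOpen: true removes all LevelMenuWidget_UI widgets and unpauses, false creates one and pauses.
; Both menu branches set cursor visibility from SetGamePaused's return value, a success flag rather than the pause state.
; ToggleCursor shows or hides the cursor, disabling look by zeroing pitch and yaw input scales while it is visible.
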(event `InputAction|OpenMenu`
  (params (Key :type "Key Structure"))
  ;[0 0 1] Univeral Opening and Closing of the Menu - Archie
  (:`Pressed`
    (bind _output_get (set `self.isMenuOpen` (not (`self.isMenuOpen`))))
    (if _output_get
      (bind _foundwidgets (`WidgetBlueprintLibrary.GetAllWidgetsOfClass` "/Game/UI/LevelMenuWidget_UI.LevelMenuWidget_UI_C"))
      (`Widget.RemoveFromParent` _foundwidgets)
      (bind _returnvalue (`GameplayStatics.SetGamePaused` false))
      (set `PlayerController.bShowMouseCursor` _returnvalue (`GameplayStatics.GetPlayerController` 0))
      (else
        (bind _returnvalue_2 (`|CreateWidget` "/Game/UI/LevelMenuWidget_UI.LevelMenuWidget_UI_C"))
        (bind _output_get_2 (set `self.ExitMenuWidget` _returnvalue_2))
        (`UserWidget.AddToViewport` _output_get_2 0)
        (bind _returnvalue_3 (`GameplayStatics.SetGamePaused` true))
        (set `PlayerController.bShowMouseCursor` _returnvalue_3 (`GameplayStatics.GetPlayerController` 0))))))

(event `InputAction|ToggleCursor`
  (params (Key :type "Key Structure"))
  (bind _returnvalue (`GameplayStatics.GetPlayerController` 0))
  ;[0 0 1] Toggle Cursor- Archie/ Jack(Rotation Disable)
  (:`Pressed`
    (bind _output_get (set `self.isCursorVisible` (not (`self.isCursorVisible`))))
    (if _output_get
      (set `PlayerController.bShowMouseCursor` true _returnvalue)
      (set `PlayerController.InputPitchScale` 0.0 _returnvalue)
      (set `PlayerController.InputYawScale` 0.0 _returnvalue)
      (else
        (set `PlayerController.bShowMouseCursor` false _returnvalue)
        (set `PlayerController.InputPitchScale` -2.5 _returnvalue)
        (set `PlayerController.InputYawScale` 2.5 _returnvalue)))))

(fn `UserConstructionScript`)