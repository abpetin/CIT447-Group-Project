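; Baby AI pawn that wanders the level, with an energy count and a happiness score.
; Construction registers it in LevelGamemode's BabyList, and a looping timer sends it to random reachable points within a radius.
; Cube hits with hazards or toys spend energy and lower or raise happiness by GameMode-tuned amounts.
; Work in progress: napping is only a debug print, and pawn-sensing events are empty.
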(event `self.ReceiveBeginPlay`
  ;[1 1 1 1 13] A baby can take a number of actions equal to 'Energy' before needing to take a nap and refill
  (set `self.Energy` 3)
  ;[1 1 1 1 13] When energy reaches 0, the baby must spend 'TimeToRefill' seconds napping to refill energy
  (set `self.TimeToRefill` (`/Game/Blueprints/Gamemodes/LevelGamemode.Nap Length` (`self.GameMode`)))
  ;[1 1 1 1 13] Each baby has a 'happiness' level that increases when they play with toys or other babies, and decreases when they are harmed by a hazard (and maybe fight with other babies if that's a thing). Happiness influences overall score.
  (set `self.Happiness` 0)
  ;[0 0 1] RANDOMIZE TIMER- ARCHIE
  (`KismetSystemLibrary.K2_SetTimerDelegate` (delegate `RandomizeTimer`) 0.0 true)
  ;[0 0 1] ARCHIE- THIS FOR BETA- KIDS WILL WANDER AROUND THEN EVENTUALLY GET TIRED, OR GET AGITATED, OR OTHER THINGS
  (`KismetSystemLibrary.K2_SetTimerDelegate` (delegate `ChildMove`) (`self.MoveTimer`) true))

(event `ChildMove`
  ;[0 0 1] ARCHIE- THIS FOR BETA- KIDS WILL WANDER AROUND THEN EVENTUALLY GET TIRED, OR GET AGITATED, OR OTHER THINGS
  (`|AIMoveTo` self (`NavigationSystemV1.K2_GetRandomReachablePointInRadius` (`self.K2_GetActorLocation`) 500.0 null null) null
    (:`then`
      ;[0 0.5 1] ARCHIE: GETTING THERE... TRY SOMETHING ELSE
      (`/Engine/EditorBlueprintResources/StandardMacros.IncrementInt` (`self.MoveInt`)))))

(event `RandomizeTimer`
  ;[0 0 1] RANDOMIZE TIMER- ARCHIE
  (set `self.MoveTimer` (`KismetMathLibrary.RandomFloatInRange` 0.5 5.0)))

(event `self.PawnSensing.OnSeePawn`
  (params (Pawn :type "Pawn Object Reference")))

(event `self.PawnSensing.OnHearNoise`
  (params (Instigator :type "Pawn Object Reference") (Location :type "Vector Structure (by ref)") (Volume :type "Float (single-precision)")))

(event `self.Cube.OnComponentHit`
  (params (HitComponent :type "PrimitiveComponent Object Reference") (OtherActor :type "Actor Object Reference") (OtherComp :type "PrimitiveComponent Object Reference") (NormalImpulse :type "Vector Structure") (Hit :type "HitResult Structure (by ref)"))
  (cast `/Game/Blueprints/Hazard_Syd` OtherActor
    (:`then`
      ;[1 1 1] When encountering a hazard, decreases the baby's energy (unless energy is already empty) and decreases happiness.
      (`self.Decrement Energy`)
      (set `self.Happiness` (- (`self.Happiness`) (`/Game/Blueprints/Gamemodes/LevelGamemode.Hazard Effect` (`self.GameMode`)))))
    (:`CastFailed`
      (cast `/Game/Blueprints/Toy_Syd` OtherActor)
      ;[1 1 1] When encountering a toy, decreases the baby's energy (unless energy is already empty) and increases happiness.
      (`self.Decrement Energy`)
      (set `self.Happiness` (+ (`self.Happiness`) (`/Game/Blueprints/Gamemodes/LevelGamemode.Toy Effect` (`self.GameMode`)))))))

(fn `Decrement Energy`
  (bind _energy (`self.Energy`))
  (if (> _energy 0)
    (set `self.Energy` (- _energy 1))
    (else
      (`KismetSystemLibrary.PrintString` "Baby state changes to sleep"))))

(fn `UserConstructionScript`
  ;[0 1 1] ARCHIE: CONTRUCTION SCRIPT TEST
  (set `self.MoveTimer` (`KismetMathLibrary.RandomFloatInRange` 1.0 10.0))
  ;[1 1 1] Gets a reference to the GameMode for the level in order to get variables changeable by the user
  (bind _aslevel_gamemode (cast `/Game/Blueprints/Gamemodes/LevelGamemode` (`GameplayStatics.GetGameMode`)))
  (bind _output_get (set `self.GameMode` _aslevel_gamemode))
  ;[1 1 1] Adds this baby to the GameMode's Baby List when this object is created.
  (bind _returnvalue (`KismetArrayLibrary.Array_Add` (`/Game/Blueprints/Gamemodes/LevelGamemode.BabyList` _output_get) self))
  ;[1 1 1] Stores this baby's array index for later ease of access
  (set `self.BabyArrayIndex` _returnvalue))