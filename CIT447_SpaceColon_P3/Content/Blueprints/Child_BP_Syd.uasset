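; Baby actor blueprint that tracks Energy and Happiness as the baby encounters hazards and toys.
; BeginPlay sets starting values, and overlaps with Hazard_Syd or Toy_Syd lower or raise Happiness respectively, both calling DecrementEnergy.
; DecrementEnergy spends energy, or only prints a sleep-state message if it is already empty.
; Napping and refill are not implemented: TimeToRefill is set but never used.
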(event `self.ReceiveBeginPlay`
  ;[1 1 1 1 13] A baby can take a number of actions equal to 'Energy' before needing to take a nap and refill
  (set `self.Energy` 3)
  ;[1 1 1 1 13] When energy reaches 0, the baby must spend 'TimeToRefill' seconds napping to refill energy
  (set `self.TimeToRefill` 10)
  ;[1 1 1 1 13] Each baby has a 'happiness' level that increases when they play with toys or other babies, and decreases when they are harmed by a hazard (and maybe fight with other babies if that's a thing). Happiness influences overall score.
  (set `self.Happiness` 0))

(event `self.ReceiveActorBeginOverlap`
  (params (OtherActor :type "Actor Object Reference"))
  (cast `/Game/Blueprints/Hazard_Syd` OtherActor
    (:`then`
      ;[1 1 1] When encountering a hazard, decreases the baby's energy (unless energy is already empty) and decreases happiness.
      (`self.DecrementEnergy`)
      (set `self.Happiness` (- (`self.Happiness`) 1)))
    (:`CastFailed`
      (cast `/Game/Blueprints/Toy_Syd` OtherActor)
      ;[1 1 1] When encountering a toy, decreases the baby's energy (unless energy is already empty) and increases happiness.
      (`self.DecrementEnergy`)
      (set `self.Happiness` (+ (`self.Happiness`) 1)))))

(fn `DecrementEnergy`
  (bind _energy (`self.Energy`))
  (if (> _energy 0)
    (set `self.Energy` (- _energy 1))
    (else
      (`KismetSystemLibrary.PrintString` "Baby state changes to sleep"))))

(fn `UserConstructionScript`)